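; Game HUD that toggles the WBP_MainMenu widget in and out of the viewport when the CloseOpenMenu input is pressed.
; ShowMenu and HideMenu lazily create and cache the widget through CreateMenu.
; Showing sets game-and-UI input focused on the menu, shows the cursor, ignores look and move, and disables player controller input.
; Hiding removes the widget and restores game-only input, hidden cursor and player control.
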(event Input|ActionEvents|InputActionCloseOpenMenu
  (params (Key :type Key%20Structure :default "None"))
  (:Pressed
    (if (UserInterface|Viewport|IsinViewport (Variables|Default|GetMenuWidget))
      (CallFunction|HideMenu)
      (else
        (CallFunction|ShowMenu)))))

(fn ConstructionScript)

(fn ShowMenu
  (bind _returnvalue (Game|Player|GetOwningPlayerController))
  (bind _menuwidget (Variables|Default|GetMenuWidget))
  (Utilities|IsValid (Variables|Default|GetMenuWidget)
    (:Is%20Valid
      _)
    (:Is%20Not%20Valid
      (CallFunction|CreateMenu)))
  (UserInterface|Viewport|AddtoViewport _menuwidget 0)
  (Input|SetInputModeGameandUI _returnvalue _menuwidget "DoNotLock" false)
  (Variables|/Script/Engine.PlayerController|SetbShowMouseCursor _returnvalue true)
  (Input|SetIgnoreLookInput _returnvalue true)
  (Input|SetIgnoreMoveInput _returnvalue true)
  (Input|DisableInput _returnvalue _returnvalue))

(fn HideMenu
  (bind _returnvalue (Game|Player|GetOwningPlayerController))
  (Utilities|IsValid (Variables|Default|GetMenuWidget)
    (:Is%20Valid
      _)
    (:Is%20Not%20Valid
      (CallFunction|CreateMenu)))
  (Widget|RemovefromParent (Variables|Default|GetMenuWidget))
  (Input|SetInputModeGameOnly _returnvalue)
  (Variables|/Script/Engine.PlayerController|SetbShowMouseCursor _returnvalue false)
  (Input|SetIgnoreLookInput _returnvalue false)
  (Input|SetIgnoreMoveInput _returnvalue false)
  (Input|EnableInput _returnvalue _returnvalue))

(fn CreateMenu
  (bind _returnvalue (UserInterface|CreateWidget "/Game/Blueprints/UI/WBP_MainMenu.WBP_MainMenu_C" (Game|Player|GetOwningPlayerController)))
  (Variables|Default|SetMenuWidget _returnvalue))