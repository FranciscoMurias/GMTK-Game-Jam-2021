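; BP_NextLevelTrigger is a level exit actor that sends the player to the level set in LevelToTravel.
; When a BP_BasePlayerCharacter overlaps it, it plays a win sound, fades the camera to full and holds it, then opens that level after the fade delay.
; Its Baloon component bobs vertically each tick on a sine of game time around the height captured at BeginPlay.
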(event EventBeginPlay
  (Variables|Default|SetHeight (.Z (Math|Vector|BreakVector (Transformation|GetWorldLocation (Variables|Default|Getbaloon))))))

(event Collision|EventActorBeginOverlap
  (params (OtherActor :type Actor%20Object%20Reference))
  (bind _returnvalue (Math|Float|MakeLiteralFloat 1.3))
  (Utilities|Casting|CastToBP_BasePlayerCharacter OtherActor)
  (Audio|PlaySound2D "/Game/SFX/SFX_LevelWin.SFX_LevelWin" 1.0 1.0 0.0 0 0)
  (CameraFades|StartCameraFade :self (Game|GetPlayerCameraManager 0) :ToAlpha 1.0 :Duration _returnvalue :bHoldWhenFinished true)
  (Utilities|FlowControl|Delay _returnvalue)
  (Game|OpenLevel(byObjectReference) (Variables|Default|GetLevelToTravel)))

(event EventTick
  (params (DeltaSeconds :type Float%20%28single-precision%29))
  (bind _baloon (Variables|Default|Getbaloon))
  (bind _returnvalue (Transformation|GetWorldLocation _baloon))
  (bind (_x _y) (Math|Vector|BreakVector _returnvalue))
  (Transformation|SetWorldLocation _baloon (Math|Vector|MakeVector _x _y (+ (* (Math|Trig|Sin(Radians) (Utilities|Time|GetTimeSeconds)) 5e+01) (Variables|Default|GetHeight))) false false))

(fn ConstructionScript)