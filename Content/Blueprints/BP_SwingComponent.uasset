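; Player controller component that lets the controlled pawn swing on a rope anchored to the player's other pawn.
; StartedSwinging spawns the rope, lowers gravity and raises the target FOV, which Tick interpolates.
; UpdateSwinging applies a pendulum-like force from anchor direction and velocity, and moves the rope end to the swinger.
; FinishedSwinging destroys the rope, restores gravity and FOV, adds a horizontal momentum launch and briefly sets JumpAfterSwing.
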(event Custom|EndJump
  (bind _as_bp_player_controller (Variables|Default|GetAs%20BP%20Player%20Controller))
  (bind _asbp_base_player_character (Utilities|Casting|CastToBP_BasePlayerCharacter (Pawn|GetControlledPawn (Variables|Default|GetAs%20BP%20Player%20Controller))))
  (Character|LaunchCharacter _asbp_base_player_character (Math|Vector|MakeVector (* (.X (Math|Vector|BreakVector (Pawn|Components|CharacterMovement|GetLastUpdateVelocity (Variables|/Script/Engine.Character|GetCharacterMovement _asbp_base_player_character)))) 0.3) (* (.Y (Math|Vector|BreakVector (Pawn|Components|CharacterMovement|GetLastUpdateVelocity (Variables|/Script/Engine.Character|GetCharacterMovement _asbp_base_player_character)))) 0.3) (* (.Z (Math|Vector|BreakVector (Pawn|Components|CharacterMovement|GetLastUpdateVelocity (Variables|/Script/Engine.Character|GetCharacterMovement _asbp_base_player_character)))) 0.0)) false false)
  (Variables|/Game/Blueprints/BP_PlayerController.BP_PlayerController_C|SetJumpAfterSwing _as_bp_player_controller true)
  (Utilities|FlowControl|RetriggerableDelay 3.0)
  (Variables|/Game/Blueprints/BP_PlayerController.BP_PlayerController_C|SetJumpAfterSwing _as_bp_player_controller false))

(event EventBeginPlay
  (bind _asbp_player_controller (Utilities|Casting|CastToBP_PlayerController (Utilities|GetOuterObject self)))
  (bind _output_get (Variables|Default|SetAs%20BP%20Player%20Controller _asbp_player_controller))
  (Development|PrintString (Utilities|GetDisplayName _output_get)))

(event EventTick
  (params (DeltaSeconds :type Float%20%28single-precision%29))
  (bind _as_bp_player_controller (Variables|Default|GetAs%20BP%20Player%20Controller))
  (bind _pawn (Default|GetCurrentPawn _as_bp_player_controller))
  (if (!= _pawn 0)
    (Variables|/Script/Engine.CameraComponent|SetFieldOfView (Variables|/Game/Blueprints/BP_BasePlayerCharacter.BP_BasePlayerCharacter_C|GetCamera (Default|GetCurrentPawn (Variables|Default|GetAs%20BP%20Player%20Controller))) (Math|Interpolation|FInterpTo (Variables|/Script/Engine.CameraComponent|GetFieldOfView (Variables|/Game/Blueprints/BP_BasePlayerCharacter.BP_BasePlayerCharacter_C|GetCamera _pawn)) (Variables|Default|GetTargetFOV) DeltaSeconds 5.0))))

(fn UpdateSwinging
  (bind _as_bp_player_controller (Variables|Default|GetAs%20BP%20Player%20Controller))
  (bind _as_bp_player_controller_2 (Variables|Default|GetAs%20BP%20Player%20Controller))
  (bind _pawn (Default|GetCurrentPawn _as_bp_player_controller))
  (bind _pawn_2 (Default|GetOtherPawn _as_bp_player_controller_2))
  (bind _returnvalue (Transformation|GetActorLocation _pawn_2))
  (bind _returnvalue_2 (Transformation|GetActorLocation _pawn))
  (bind _charactermovement (Variables|/Script/Engine.Character|GetCharacterMovement _pawn))
  (bind _returnvalue_3 (- _returnvalue _returnvalue_2))
  (Physics|AddForce _charactermovement (* (+ (* (Math|Vector|ClampVectorSize (- (Transformation|GetActorLocation (Default|GetOtherPawn (Variables|Default|GetAs%20BP%20Player%20Controller))) (Transformation|GetActorLocation (Default|GetCurrentPawn (Variables|Default|GetAs%20BP%20Player%20Controller)))) 0.0 8e+02) 1e+03) (* (* (* (Math|Vector|Normalize _returnvalue_3) (Math|Vector|DotProduct (Math|Vector|ClampVectorSize _returnvalue_3 -1e+03 1e+03) (Math|Vector|ClampVectorSize (Variables|/Script/Engine.MovementComponent|GetVelocity _charactermovement) -8e+02 8e+02))) -2.0) 2.0)) 1.0))
  (Transformation|SetWorldLocation (Variables|/Game/Blueprints/BP_Rope.BP_Rope_C|GetTarget (Variables|Default|GetRope)) (Transformation|GetActorLocation (Default|GetCurrentPawn (Variables|Default|GetAs%20BP%20Player%20Controller))) false true))

(fn StartedSwinging
  (bind _as_bp_player_controller (Variables|Default|GetAs%20BP%20Player%20Controller))
  (bind _pawn (Default|GetOtherPawn _as_bp_player_controller))
  (Audio|PlaySound2D "/Game/SFX/SFX_Swing_Temporary.SFX_Swing_Temporary" 1.0 1.0 0.0 0 0)
  (bind _returnvalue (Game|SpawnActorfromClass "/Game/Blueprints/BP_Rope.BP_Rope_C" (Math|Transform|MakeTransform (Transformation|GetActorLocation _pawn) "0, 0, 0" "1,1,1") "Undefined" _pawn (Default|GetCurrentPawn _as_bp_player_controller)))
  (bind _output_get (Variables|Default|SetRope _returnvalue))
  (Transformation|AttachActorToActor _output_get _pawn "None" "SnapToTarget" "KeepRelative" "KeepRelative" true)
  (Variables|/Script/Engine.CharacterMovementComponent|SetGravityScale (Variables|/Script/Engine.Character|GetCharacterMovement (Default|GetCurrentPawn (Variables|Default|GetAs%20BP%20Player%20Controller))) 1.0)
  (Variables|Default|SetTargetFOV (+ (Variables|Default|GetBaseFOV) (Variables|Default|GetTargetIncreaseFOV)))
  (Development|PrintString "Started swinging"))

(fn FinishedSwinging
  (CallFunction|EndJump)
  (Actor|DestroyActor (Variables|Default|GetRope))
  (Variables|/Script/Engine.CharacterMovementComponent|SetGravityScale (Variables|/Script/Engine.Character|GetCharacterMovement (Default|GetCurrentPawn (Variables|Default|GetAs%20BP%20Player%20Controller))) 3.0)
  (Variables|Default|SetTargetFOV (Variables|Default|GetBaseFOV))
  (Development|PrintString "Finished swinging"))