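; Feather pickup that resets the player's power through BP_PlayerController when BP_BasePlayerCharacter overlaps its Box.
; A PickedUp flag blocks repeat triggers while the feather is hidden, and a temporary Niagara effect is destroyed after a short delay.
; The actor is never destroyed: the RespawnFeather event clears the flag and shows the feather again, with no caller in this Blueprint.
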(event OnComponentBeginOverlap(Box)
  (params (OverlappedComponent :type Primitive%20Component%20Object%20Reference) (OtherActor :type Actor%20Object%20Reference) (OtherComp :type Primitive%20Component%20Object%20Reference) (OtherBodyIndex :type Integer) (bFromSweep :type Boolean) (SweepResult :type Hit%20Result%20Structure%20%28by%20ref%29))
  (Utilities|Casting|CastToBP_BasePlayerCharacter OtherActor)
  (if (not (Variables|Default|GetPicked%20up))
    (Variables|Default|SetPicked%20up true)
    (bind _asbp_player_controller (Utilities|Casting|CastToBP_PlayerController (Game|GetPlayerController 0)))
    (Default|ResetPower _asbp_player_controller)
    (bind _returnvalue (AddComponent|AddNiagaraComponent false))
    (Rendering|SetVisibility (Variables|Default|Getfeather) false false)
    (Utilities|FlowControl|Delay 3.0)
    (Components|DestroyComponent _returnvalue)))

(event Custom|RespawnFeather
  (if (Variables|Default|GetPicked%20up)
    (Variables|Default|SetPicked%20up false)
    (Rendering|SetVisibility (Variables|Default|Getfeather) true false)))

(event EventBeginPlay)

(event Collision|EventActorBeginOverlap
  (params (OtherActor :type Actor%20Object%20Reference)))

(event EventTick
  (params (DeltaSeconds :type Float%20%28single-precision%29)))

(fn ConstructionScript)