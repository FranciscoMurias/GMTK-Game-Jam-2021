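; Game mode for a game where one player controller owns two characters, handling startup, spawning and checkpoint respawns.
; A new player sees the menu through a "Start"-tagged camera, or starts immediately if none exists.
; Spawning registers checkpoint zones tagged "First" and "Second", then creates each character at its zone's spawn point.
; Respawn fades the screen out, teleports both characters to their registered checkpoints, zeroes velocity and fades back in.
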(event Custom|RespawnAtCheckpoint
  (bind _transform (CallFunction|GetSecondSpawnTransform))
  (bind _transform_2 (CallFunction|GetFirstSpawnTransform))
  (bind _as_bp_player_controller (Variables|Default|GetAs%20BP%20Player%20Controller))
  (bind _firstpawn (Variables|/Game/Blueprints/BP_PlayerController.BP_PlayerController_C|GetFirstPawn _as_bp_player_controller))
  (bind _secondpawn (Variables|/Game/Blueprints/BP_PlayerController.BP_PlayerController_C|GetSecondPawn _as_bp_player_controller))
  (CameraFades|StartCameraFade (Game|GetPlayerCameraManager 0) 0.0 1.0 0.5 (Variables|Default|GetFadeColor) false true)
  (Utilities|FlowControl|Delay 0.5)
  (Utilities|FlowControl|Sequence
    (:then_1
      ;[1 1 1] Todo need to do something with camera or just fade in fade out
      (Transformation|Teleport _firstpawn (.location _transform_2) (.rotation _transform_2))
      (Variables|/Script/Engine.MovementComponent|SetVelocity (Variables|/Script/Engine.Character|GetCharacterMovement _firstpawn) "0, 0, 0"))
    (:then_2
      (Transformation|Teleport _secondpawn (.location _transform) (.rotation _transform))
      (Variables|/Script/Engine.MovementComponent|SetVelocity (Variables|/Script/Engine.Character|GetCharacterMovement _secondpawn) "0, 0, 0"))
    (:then_3
      (CameraFades|StartCameraFade (Game|GetPlayerCameraManager 0) 1.0 0.0 1.0 (Variables|Default|GetFadeColor) false false))))

(event Custom|SpawnChars
  (params (NewPlayer :type Player%20Controller%20Object%20Reference))
  (Utilities|FlowControl|Sequence
    (:then_0
      (bind _outactors (Actor|GetAllActorsOfClasswithTag "/Game/Blueprints/Gameplay/BP_CheckpointZone.BP_CheckpointZone_C" "First"))
      (CallFunction|RegisterCheckPointforFirst (Utilities|Array|Get(acopy) _outactors)))
    (:then_1
      (bind _outactors_2 (Actor|GetAllActorsOfClasswithTag "/Game/Blueprints/Gameplay/BP_CheckpointZone.BP_CheckpointZone_C" "Second"))
      (CallFunction|RegisterCheckPointforSecond (Utilities|Array|Get(acopy) _outactors_2)))
    (:then_2
      (bind _returnvalue (Game|SpawnActorfromClass "/Game/Blueprints/BP_FirstCharacter.BP_FirstCharacter_C" (CallFunction|GetFirstSpawnTransform) "Undefined" (Variables|Default|GetAs%20BP%20Player%20Controller) 0))
      (Variables|/Game/Blueprints/BP_PlayerController.BP_PlayerController_C|SetFirstPawn (Variables|Default|GetAs%20BP%20Player%20Controller) _returnvalue))
    (:then_3
      (bind _returnvalue_2 (Game|SpawnActorfromClass "/Game/Blueprints/BP_SecondCharacter.BP_SecondCharacter_C" (CallFunction|GetSecondSpawnTransform) "Undefined" (Variables|Default|GetAs%20BP%20Player%20Controller) 0))
      (Variables|/Game/Blueprints/BP_PlayerController.BP_PlayerController_C|SetSecondPawn (Variables|Default|GetAs%20BP%20Player%20Controller) _returnvalue_2))))

(event EventBeginPlay
  (bind _returnvalue (AddComponent|AddAudioComponent false))
  (Audio|Components|Audio|FadeIn _returnvalue 1.0 1.0 0.0 "Linear" :!class /Script/Engine.AudioComponent))

(event EventHandleStartingNewPlayer
  (params (NewPlayer :type Player%20Controller%20Object%20Reference))
  (bind _asbp_player_controller (Utilities|Casting|CastToBP_PlayerController NewPlayer))
  (bind _output_get (Variables|Default|SetAs%20BP%20Player%20Controller _asbp_player_controller))
  (bind _asbp_hud_game (Utilities|Casting|CastToBP_HUD_Game (HUD|GetHUD _output_get)))
  (bind _output_get_2 (Variables|Default|SetHUD _asbp_hud_game))
  (Input|EnableInput _output_get_2 _output_get)
  (bind _outactors (Actor|GetAllActorsOfClasswithTag "/Script/Engine.CameraActor" "Start"))
  (if (>= (Utilities|Array|Length _outactors) 1)
    (Default|ShowMenu (Variables|Default|GetHUD))
    (Game|Player|SetViewTargetwithBlend (Game|GetPlayerController 0) (Utilities|Array|Get(acopy) _outactors) 0.0 "VTBlend_Linear" 0.0 false)
    (else
      (CallFunction|SpawnChars (Variables|Default|GetAs%20BP%20Player%20Controller))
      (Default|StartGame (Variables|Default|GetAs%20BP%20Player%20Controller))
      (Default|HideMenu (Variables|Default|GetHUD)))))

(fn ConstructionScript)

(fn GetFirstSpawnTransform
  (bind _firstpawncheckpoint (Variables|Default|GetFirstPawnCheckpoint))
  (bind _firstspawn (Variables|/Game/Blueprints/Gameplay/BP_CheckpointZone.BP_CheckpointZone_C|GetFirstSpawn _firstpawncheckpoint))
  (bind _returnvalue (Transformation|GetWorldTransform _firstspawn))
  (Utilities|IsValid _firstpawncheckpoint
    (:Is%20Valid
      (return (Math|Transform|MakeTransform (.location _returnvalue) (.rotation _returnvalue) "1,1,1")))
    (:Is%20Not%20Valid
      (Development|PrintString "cound not find BP_SpawnPoint_FirstCharacter")
      (return ""))))

(fn GetSecondSpawnTransform
  (bind _secondpawncheckpoint (Variables|Default|GetSecondPawnCheckpoint))
  (bind _secondspawn (Variables|/Game/Blueprints/Gameplay/BP_CheckpointZone.BP_CheckpointZone_C|GetSecondSpawn _secondpawncheckpoint))
  (bind _returnvalue (Transformation|GetWorldTransform _secondspawn))
  (Utilities|IsValid _secondpawncheckpoint
    (:Is%20Valid
      (return (Math|Transform|MakeTransform (.location _returnvalue) (.rotation _returnvalue) "1,1,1")))
    (:Is%20Not%20Valid
      (Development|PrintString "Add to one of checkpoint zone tag \"Second\"")
      (return ""))))

(fn RegisterCheckPointforFirst
  (params (Checkpoint :type BP%20Checkpoint%20Zone%20Object%20Reference))
  (Variables|Default|SetFirstPawnCheckpoint Checkpoint))

(fn RegisterCheckPointforSecond
  (params (Checkpoint :type BP%20Checkpoint%20Zone%20Object%20Reference))
  (Variables|Default|SetSecondPawnCheckpoint Checkpoint))

(fn StartGame
  (bind _as_bp_player_controller (Variables|Default|GetAs%20BP%20Player%20Controller))
  (CallFunction|SpawnChars _as_bp_player_controller)
  (Default|StartGame _as_bp_player_controller)
  (Default|HideMenu (Variables|Default|GetHUD)))